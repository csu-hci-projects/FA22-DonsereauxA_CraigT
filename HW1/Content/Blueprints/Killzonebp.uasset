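; Kill zone volume that kills and respawns the bpSphere player when it enters the Overlap box.
; On overlap it deducts score, plays a death sound, zeroes player health, then calls Respawn on the sphere after a short delay.
; The construction script sizes the box from the InBoxExtent variable, so each placed zone can have its own extent.
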(event `self.Overlap.OnComponentBeginOverlap`
  (params (OverlappedComponent :type "PrimitiveComponent Object Reference") (OtherActor :type "Actor Object Reference") (OtherComp :type "PrimitiveComponent Object Reference") (OtherBodyIndex :type Integer) (bFromSweep :type Boolean) (SweepResult :type "HitResult Structure (by ref)"))
  (bind _asbp_sphere (cast `/Game/Blueprints/bpSphere` OtherActor))
  (set `/Game/Blueprints/bpSphere.Score` (- (`/Game/Blueprints/bpSphere.Score` _asbp_sphere) 10) _asbp_sphere)
  (`GameplayStatics.PlaySound2D` "/Game/RetroSoundEffects1/Wavs/Death_1.Death_1" 1.0 1.0 0.0 null null)
  (set `/Game/Blueprints/bpSphere.PlayerHealth` 0.0 _asbp_sphere)
  (`KismetSystemLibrary.Delay` 1.0)
  (`/Game/Blueprints/bpSphere.Respawn` _asbp_sphere))

(fn `UserConstructionScript`
  (`BoxComponent.SetBoxExtent` (`self.Overlap`) (`self.In Box Extent`) true))