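; An actor that moves back and forth along a Direction vector, reversing at a regular interval.
; On BeginPlay a looping timer fires ChangeDirection every TimeToChange seconds, which negates Direction.
; Tick offsets the actor by the normalized Direction scaled by Speed and delta time, without sweep, so movement is frame-rate independent and ignores collision.
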(event `self.ReceiveBeginPlay`
  ;[1 1 1] Every Time to change, call ChangeDireciton
  (`KismetSystemLibrary.K2_SetTimerDelegate` (delegate `ChangeDirection`) (`self.TimeToChange`) true))

(event `ChangeDirection`
  ;[1 1 1] Flips direction
  (set `self.Direction` (* (`self.Direction`) -1.0)))

(event `self.ReceiveTick`
  (params (DeltaSeconds :type "Float (single-precision)"))
  ;[1 1 1] Every frame, update location
  (`self.K2_AddActorWorldOffset` (* (`KismetMathLibrary.Normal` (`self.Direction`)) (* (`self.Speed`) (`GameplayStatics.GetWorldDeltaSeconds`)))))

(fn `UserConstructionScript`)