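; NextLevelBp is a level-exit trigger that advances the game to the next numbered level when a bpSphere overlaps its NextLvlOverlap box.
; It plays a reward sound, waits briefly, then opens "Level" plus the current number incremented by one.
; The number comes from the single character at index 5 of the current level name, so only one digit is read.
; The construction script sizes the box from the InBoxExtentlvl variable.
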(event `self.NextLvlOverlap.OnComponentBeginOverlap`
  (params (OverlappedComponent :type "PrimitiveComponent Object Reference") (OtherActor :type "Actor Object Reference") (OtherComp :type "PrimitiveComponent Object Reference") (OtherBodyIndex :type Integer) (bFromSweep :type Boolean) (SweepResult :type "HitResult Structure (by ref)"))
  (cast `/Game/Blueprints/bpSphere` OtherActor
    (:`then`
      (`GameplayStatics.PlaySound2D` "/Game/RetroSoundFX/wav/S_RetroSoundFX_GloriousRewardA_1.S_RetroSoundFX_GloriousRewardA_1" 1.0 1.0 0.0 null null)
      (`KismetSystemLibrary.Delay` 0.75)
      (bind _returnvalue (`GameplayStatics.GetCurrentLevelName` true))
      (bind _output_get (set `self.lvlName` (`KismetStringLibrary.Concat_StrStr` "Level" (`KismetStringLibrary.Conv_IntToString` (+ (`KismetStringLibrary.Conv_StringToInt` (`KismetStringLibrary.GetSubstring` _returnvalue 5)) 1)))))
      (`GameplayStatics.OpenLevel` (`KismetStringLibrary.Conv_StringToName` _output_get)))
    (:`CastFailed`
      (`KismetSystemLibrary.PrintString` "Failed"))))

(fn `UserConstructionScript`
  (`BoxComponent.SetBoxExtent` (`self.NextLvlOverlap`) (`self.In Box Extentlvl`) true))