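; Moving obstacle that patrols back and forth and forces a respawn when it hits a bpSphere actor.
; Tick offsets it along the normalized Direction at Speed without sweeping, and a looping timer reverses Direction every TimeToChange seconds.
; On Hit, a successful bpSphere cast plays a hurt sound, destroys this actor and calls Respawn on that sphere; other hits print a failure message.
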(event `self.ReceiveHit`
  (params (MyComp :type "PrimitiveComponent Object Reference") (Other :type "Actor Object Reference") (OtherComp :type "PrimitiveComponent Object Reference") (bSelfMoved :type Boolean) (HitLocation :type "Vector Structure") (HitNormal :type "Vector Structure") (NormalImpulse :type "Vector Structure") (Hit :type "HitResult Structure (by ref)"))
  (bind _asbp_sphere (cast `/Game/Blueprints/bpSphere` Other)
    (:`then`
      (`GameplayStatics.PlaySound2D` "/Game/RetroSoundEffects1/Wavs/Hurt_1.Hurt_1" 1.0 1.0 0.0 null null)
      (`self.K2_DestroyActor`)
      (`/Game/Blueprints/bpSphere.Respawn` _asbp_sphere))
    (:`CastFailed`
      (`KismetSystemLibrary.PrintString` "Failed"))))

(event `self.ReceiveTick`
  (params (DeltaSeconds :type "Float (single-precision)"))
  (`self.K2_AddActorWorldOffset` (* (`KismetMathLibrary.Normal` (`self.Direction`)) (* (`self.speed`) (`GameplayStatics.GetWorldDeltaSeconds`)))))

(event `self.ReceiveBeginPlay`
  (`KismetSystemLibrary.K2_SetTimerDelegate` (delegate `ChangeDirection`) (`self.TimeToChange`) true))

(event `ChangeDirection`
  (set `self.Direction` (* (`self.Direction`) -1.0)))

(fn `UserConstructionScript`)