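; bpCoin is a collectible coin that awards score when the bpSphere ball overlaps it.
; On overlap it adds 100 to the ball's Score, copies that total to the PersistentScore game instance, then plays a sound and destroys itself.
; The score copy, sound and destruction only run if the game instance cast succeeds.
; Tick spins the coin by a fixed rotation each frame, independent of delta time.
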(event `self.ReceiveBeginPlay`)

(event `self.ReceiveActorBeginOverlap`
  (params (OtherActor :type "Actor Object Reference"))
  ;[1 1 1] On overlap with ball
  (bind _asbp_sphere (cast `/Game/Blueprints/bpSphere` OtherActor))
  ;[1 1 1] Set Score +100
  (bind _output_get (set `/Game/Blueprints/bpSphere.Score` (+ (`/Game/Blueprints/bpSphere.Score` _asbp_sphere) 100) _asbp_sphere))
  (bind _aspersistent_score (cast `/Game/Blueprints/PersistentScore` (`GameplayStatics.GetGameInstance`)))
  (set `/Game/Blueprints/PersistentScore.PlayerScore` _output_get _aspersistent_score)
  ;[1 1 1] Play coin sound
  (`GameplayStatics.PlaySoundAtLocation` "/Game/RetroSoundEffects1/Wavs/Coin_1.Coin_1" (`self.K2_GetActorLocation`) (struct) 1.0 1.0 0.0 null null null null)
  ;[1 1 1] Remove coin
  (`self.K2_DestroyActor`))

(event `self.ReceiveTick`
  (params (DeltaSeconds :type "Float (single-precision)"))
  ;[1 1 1] Coin rotation
  (`self.K2_SetActorRotation` (`KismetMathLibrary.ComposeRotators` (`self.K2_GetActorRotation`) (struct :`Yaw` 1.0))))

(fn `UserConstructionScript`)