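; Health pickup actor that restores health to the bpSphere player when it overlaps.
; It adds a fixed amount clamped to a hardcoded 100 rather than MaxHealth, playing a different sound for low, higher or full health.
; The pickup destroys itself even at full health; other overlapping actors only print a debug string.
; Tick spins it by a fixed step each frame, independent of delta time.
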(event `self.ReceiveActorBeginOverlap`
  (params (OtherActor :type "Actor Object Reference"))
  (bind _asbp_sphere (cast `/Game/Blueprints/bpSphere` OtherActor)
    (:`then`
      (bind _playerhealth (`/Game/Blueprints/bpSphere.PlayerHealth` _asbp_sphere))
      (if (== _playerhealth (`/Game/Blueprints/bpSphere.MaxHealth` _asbp_sphere))
        (`GameplayStatics.PlaySound2D` "/Game/RetroSoundEffects1/Wavs/ExtraLife_1.ExtraLife_1" 1.0 1.0 0.0 null null)
        (`self.K2_DestroyActor`)
        (else
          (if (< _playerhealth 50.0)
            (`GameplayStatics.PlaySound2D` "/Game/RetroSoundEffects1/Wavs/ExtraLife_3.ExtraLife_3" 1.0 1.0 0.0 null null)
            (bind _returnvalue (`KismetMathLibrary.FClamp` (+ (`/Game/Blueprints/bpSphere.PlayerHealth` _asbp_sphere) 50.0) 0.0 100.0))
            (set `/Game/Blueprints/bpSphere.PlayerHealth` _returnvalue _asbp_sphere)
            (else
              (`GameplayStatics.PlaySound2D` "/Game/RetroSoundEffects1/Wavs/ExtraLife_2.ExtraLife_2" 1.0 1.0 0.0 null null)
              (set `/Game/Blueprints/bpSphere.PlayerHealth` _returnvalue _asbp_sphere)))
          (`self.K2_DestroyActor`))))
    (:`CastFailed`
      (`KismetSystemLibrary.PrintString` "FailedHealth"))))

(event `self.ReceiveTick`
  (params (DeltaSeconds :type "Float (single-precision)"))
  (`self.K2_SetActorRotation` (`KismetMathLibrary.ComposeRotators` (`self.K2_GetActorRotation`) (struct :`Yaw` 1.0))))

(fn `UserConstructionScript`)