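; Bomb hazard actor that penalizes the player's bpSphere ball when the two overlap.
; On overlap it subtracts score, clamped at zero, reduces player health and copies the new score to the PersistentScore game instance.
; It then plays an explosion sound at the ball, destroys itself and also destroys the ball if its health is depleted.
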(event `self.ReceiveActorBeginOverlap`
  (params (OtherActor :type "Actor Object Reference"))
  ;[1 1 1] On overlap with ball
  (bind _asbp_sphere (cast `/Game/Blueprints/bpSphere` OtherActor))
  (bind _returnvalue (- (`/Game/Blueprints/bpSphere.Score` _asbp_sphere) 200))
  ;[1 1 1] Set Score -1000 (until 0)
  (if (< _returnvalue 0)
    (set `/Game/Blueprints/bpSphere.Score` 0 _asbp_sphere)
    (else
      (bind _output_get (set `/Game/Blueprints/bpSphere.Score` _returnvalue _asbp_sphere))))
  (bind _output_get_2 (set `/Game/Blueprints/bpSphere.PlayerHealth` (- (`/Game/Blueprints/bpSphere.PlayerHealth` _asbp_sphere) 50.0) _asbp_sphere))
  (bind _aspersistent_score (cast `/Game/Blueprints/PersistentScore` (`GameplayStatics.GetGameInstance`)))
  (set `/Game/Blueprints/PersistentScore.PlayerScore` _output_get _aspersistent_score)
  ;[1 1 1] Play bomb sound
  (`GameplayStatics.PlaySoundAtLocation` "/Game/RetroSoundEffects1/Wavs/Explosion_1.Explosion_1" (`self.K2_GetActorLocation` _asbp_sphere) (struct) 1.0 1.0 0.0 null null null null)
  ;[1 1 1] Remove bomb
  (`self.K2_DestroyActor`)
  (if (<= _output_get_2 0.0)
    (`self.K2_DestroyActor` _asbp_sphere)))

(fn `UserConstructionScript`)