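; An early or old player-controlled rolling ball that moves with physics and can jump.
; The MoveXaxis and MoveYaxis inputs share one torque call on the sphere mesh, applied as an acceleration change around X and Y.
; Jump applies an upward velocity impulse with a sound and clears CanJump.
; Any hit re-enables jumping, playing an impact sound if the ball had jumped, with no floor check.
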(event `InputAxis|MoveYaxis`
  (params (AxisValue :type "Float (single-precision)"))
  ;[1 1 1] Move X&Y Axis
  (`PrimitiveComponent.AddTorqueInDegrees` (`self.SphereStaticMesh`) (`KismetMathLibrary.MakeVector` (* (stale `InputAxis|MoveXaxis` AxisValue) (`self.TorqueValue`)) (* AxisValue (`self.TorqueValue`))) "None" true :!label _label))

(event `InputAxis|MoveXaxis`
  (params (AxisValue :type "Float (single-precision)"))
  ;[1 1 1] Move X&Y Axis
  (goto _label))

(event `InputAction|Jump`
  (params (Key :type "Key Structure"))
  (:`Pressed`
    (if (`self.CanJump`)
      (`PrimitiveComponent.AddImpulse` (`self.SphereStaticMesh`) (`KismetMathLibrary.MakeVector` 0.0 0.0 (`self.ImpulseValue`)) "None" true)
      (set `self.CanJump` false)
      (`GameplayStatics.PlaySound2D` "/Game/RetroSoundEffects1/Cues/Jump_5_Cue.Jump_5_Cue" 1.0 1.0 0.0 null null))))

(event `self.ReceiveHit`
  (params (MyComp :type "PrimitiveComponent Object Reference") (Other :type "Actor Object Reference") (OtherComp :type "PrimitiveComponent Object Reference") (bSelfMoved :type Boolean) (HitLocation :type "Vector Structure") (HitNormal :type "Vector Structure") (NormalImpulse :type "Vector Structure") (Hit :type "HitResult Structure (by ref)"))
  (if (not (`self.CanJump`))
    (`GameplayStatics.PlaySound2D` "/Game/Retro_8Bit_Sounds/Impacts/Wavs/retro_impact_hit_11.retro_impact_hit_11" 1.0 1.0 0.0 null null))
  (set `self.CanJump` true))

(fn `UserConstructionScript`)